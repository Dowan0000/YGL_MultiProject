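; Rifle ammo pickup that adds reserve rounds to a MainCharacter who walks into its box trigger.
; The overlap runs only on authority and requires the character to have a rifle.
; It raises MaxAmmo on the second inventory slot by a fixed amount, clamped to a cap, then destroys itself, even if the ammo was already full.
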(event OnComponentBeginOverlap(Box)
  (params (OverlappedComponent :type Primitive%20Component%20Object%20Reference) (OtherActor :type Actor%20Object%20Reference) (OtherComp :type Primitive%20Component%20Object%20Reference) (OtherBodyIndex :type Integer) (bFromSweep :type Boolean) (SweepResult :type Hit%20Result%20Structure%20%28by%20ref%29))
  (Networking|SwitchHasAuthority
    (:Authority
      (bind _asmain_character (Utilities|Casting|CastToMainCharacter OtherActor))
      (if (Variables|/Script/YGL_MultiProject.MainCharacter|GetHasRifle _asmain_character)
        (Variables|/Script/YGL_MultiProject.WeaponBase|SetMaxAmmo (Utilities|Array|Get(acopy) (Variables|/Script/YGL_MultiProject.MainCharacter|GetInventory _asmain_character) 1) (Math|Integer|Clamp(Integer) (+ (Variables|/Script/YGL_MultiProject.WeaponBase|GetMaxAmmo (Utilities|Array|Get(acopy) (Variables|/Script/YGL_MultiProject.MainCharacter|GetInventory _asmain_character) 1)) 30) 0 150))
        (Actor|DestroyActor)))))

(fn ConstructionScript)