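; BP_MainCharacter_A is a playable character that can enter and exit an SUV, focus chat and open a pause menu.
; Capsule overlaps with BPI_Interaction2 actors cache the SUV and flag it as available.
; ExitVehicle toggles riding: entry calls OnInteractedMessage through VehicleServer and VehicleMul, while exit detaches the character, restores collision and visibility, and frees Seat2.
; ChattingEnter focuses the HUD's chat box, and Escape spawns the pause widget, both using UI-only input.
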(event OnComponentBeginOverlap(CapsuleComponent)
  (params (OverlappedComponent :type Primitive%20Component%20Object%20Reference) (OtherActor :type Actor%20Object%20Reference) (OtherComp :type Primitive%20Component%20Object%20Reference) (OtherBodyIndex :type Integer) (bFromSweep :type Boolean) (SweepResult :type Hit%20Result%20Structure%20%28by%20ref%29))
  (if (Utilities|DoesObjectImplementInterface OtherActor "/Game/_Dowan/Vehicle/BPI_Interaction2.BPI_Interaction2_C")
    (bind _asbp_vehicle_suv (Utilities|Casting|CastToBP_Vehicle_SUV OtherActor))
    (Variables|Default|SetAs%20BP%20Vehicle%20SUV _asbp_vehicle_suv)
    (Variables|Default|SetVehicletest true)))

(event OnComponentEndOverlap(CapsuleComponent)
  (params (OverlappedComponent :type Primitive%20Component%20Object%20Reference) (OtherActor :type Actor%20Object%20Reference) (OtherComp :type Primitive%20Component%20Object%20Reference) (OtherBodyIndex :type Integer))
  (if (Utilities|DoesObjectImplementInterface OtherActor "/Game/_Dowan/Vehicle/BPI_Interaction2.BPI_Interaction2_C")
    (Variables|Default|SetAs%20BP%20Vehicle%20SUV 0)
    (Variables|Default|SetVehicletest false)))

(event Custom|VehicleMul
  (Class|BPIInteraction2|OnInteracted(Message) (stale OnComponentBeginOverlap(CapsuleComponent) OtherActor) self))

(event Custom|VehicleServer
  (CallFunction|VehicleMul))

(event EventBeginPlay)

(event Input|ActionEvents|InputActionChattingEnter
  (params (Key :type Key%20Structure :default "None"))
  (:Pressed
    (bind _asbp_main_hud (Utilities|Casting|CastToBP_MainHUD (HUD|GetHUD (Game|GetPlayerController 0))))
    (if (not (Class|Widget|HasKeyboardFocus (Variables|/Game/_HyeChang/Widgets/WB_Chat.WB_Chat_C|GetChatMessage_InputBox (Variables|/Game/_Dowan/UI/BP_MainHUD.BP_MainHUD_C|GetWBChatRef _asbp_main_hud))))
      (Input|SetInputModeUIOnly (Game|GetPlayerController 0) (Variables|/Game/_HyeChang/Widgets/WB_Chat.WB_Chat_C|GetChatMessage_InputBox (Variables|/Game/_Dowan/UI/BP_MainHUD.BP_MainHUD_C|GetWBChatRef _asbp_main_hud)) "DoNotLock"))))

(event Input|ActionEvents|InputActionExitVehicle
  (params (Key :type Key%20Structure :default "None"))
  (:Pressed
    (if (Variables|Default|GetInCar)
      (Collision|SetActorEnableCollision true)
      (Rendering|SetActorHiddenInGame false)
      (Transformation|DetachFromActor "KeepWorld" "KeepWorld" "KeepWorld")
      (Variables|Default|SetInCar false)
      (Variables|/Game/_Dowan/Vehicle/BP_Vehicle_SUV.BP_Vehicle_SUV_C|SetSeat2 (Variables|Default|GetAs%20BP%20Vehicle%20SUV) false)
      (elif (Variables|Default|GetVehicletest)
        (Variables|Default|SetInCar true)
        (CallFunction|VehicleServer)))))

(event Input|KeyboardEvents|Escape
  (params (Key :type Key%20Structure :default "None"))
  (bind _returnvalue (Game|GetPlayerController 0))
  (:Pressed
    (bind _returnvalue_2 (UserInterface|CreateWidget "/Game/_HyeChang/Widgets/GamePauseMenuWidget.GamePauseMenuWidget_C"))
    (Variables|/Script/Engine.PlayerController|SetbShowMouseCursor _returnvalue true)
    (Input|SetInputModeUIOnly _returnvalue _returnvalue_2 "DoNotLock")
    (UserInterface|Viewport|AddtoViewport _returnvalue_2 0)))

(fn ConstructionScript)