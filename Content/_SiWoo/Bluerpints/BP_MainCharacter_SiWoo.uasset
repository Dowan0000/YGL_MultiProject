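; Player character Blueprint that links the character to the main HUD and triggers interactions on contact.
; BeginPlay runs the parent logic, then creates WBP_MainUI and adds it to the viewport.
; SetWeaponUI passes the character to four weapon slot widgets and shows the equipped weapon's row name in the ammo counter widget.
; Capsule overlaps send an interaction message to any actor implementing BPI_Interaction.
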(event OnComponentBeginOverlap(CapsuleComponent)
  (params (OverlappedComponent :type Primitive%20Component%20Object%20Reference) (OtherActor :type Actor%20Object%20Reference) (OtherComp :type Primitive%20Component%20Object%20Reference) (OtherBodyIndex :type Integer) (bFromSweep :type Boolean) (SweepResult :type Hit%20Result%20Structure%20%28by%20ref%29))
  (if (Utilities|DoesObjectImplementInterface OtherActor "/Game/_SiWoo/Vehicle/BPI_Interaction.BPI_Interaction_C")
    (Class|BPIInteraction|OnInteracted(Message) OtherActor)))

(event EventBeginPlay
  ;[1 1 1] MainUI 불러오기
  (|CallParentFunction)
  (bind _returnvalue (UserInterface|CreateWidget "/Game/_DongJin/WBP_MainUI.WBP_MainUI_C"))
  (bind _output_get (Variables|Default|SetMainUI _returnvalue))
  (UserInterface|Viewport|AddtoViewport _output_get 0))

(event EventSetWeaponUI
  (Utilities|FlowControl|Sequence
    (:then_0
      (Default|SetCharacter (Variables|/Game/_DongJin/WBP_WeaponSlotInventroy.WBP_WeaponSlotInventroy_C|GetWBP_WeaponSlot (Variables|/Game/_DongJin/WBP_MainUI.WBP_MainUI_C|GetWBP_WeaponSlotInventroy (Variables|Default|GetMainUI))) self))
    (:then_1
      (Default|SetCharacter (Variables|/Game/_DongJin/WBP_WeaponSlotInventroy.WBP_WeaponSlotInventroy_C|GetWBP_WeaponSlot_0 (Variables|/Game/_DongJin/WBP_MainUI.WBP_MainUI_C|GetWBP_WeaponSlotInventroy (Variables|Default|GetMainUI))) self))
    (:then_2
      (Default|SetCharacter (Variables|/Game/_DongJin/WBP_WeaponSlotInventroy.WBP_WeaponSlotInventroy_C|GetWBP_WeaponSlot_1 (Variables|/Game/_DongJin/WBP_MainUI.WBP_MainUI_C|GetWBP_WeaponSlotInventroy (Variables|Default|GetMainUI))) self))
    (:then_3
      (Default|SetCharacter (Variables|/Game/_DongJin/WBP_WeaponSlotInventroy.WBP_WeaponSlotInventroy_C|GetWBP_WeaponSlot_2 (Variables|/Game/_DongJin/WBP_MainUI.WBP_MainUI_C|GetWBP_WeaponSlotInventroy (Variables|Default|GetMainUI))) self))
    (:then_4
      (Default|SetWeaponName (Variables|/Game/_DongJin/WBP_WeaponSlotInventroy.WBP_WeaponSlotInventroy_C|GetWBP_AmmoCount (Variables|/Game/_DongJin/WBP_MainUI.WBP_MainUI_C|GetWBP_WeaponSlotInventroy (Variables|Default|GetMainUI))) (Utilities|Text|ToText(Name) (Variables|/Script/YGL_MultiProject.WeaponBase|GetRowName (Variables|Default|GetEquipWeapon)))))))

(fn ConstructionScript)