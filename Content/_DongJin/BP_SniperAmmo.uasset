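; BP_SniperAmmo is a sniper ammo pickup that increases a character's maximum ammo when touched.
; On server-side sphere overlap with BP_MainCharacterDongJin, it rebuilds MaxAmmo as three entries, deriving the third from index 3, not 2, plus a fixed bonus.
; It then refreshes ammo UI through player controller 0's HUD, rather than the overlapping player's, and destroys itself only if that HUD cast succeeds.
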(event OnComponentBeginOverlap(Sphere)
  (params (OverlappedComponent :type Primitive%20Component%20Object%20Reference) (OtherActor :type Actor%20Object%20Reference) (OtherComp :type Primitive%20Component%20Object%20Reference) (OtherBodyIndex :type Integer) (bFromSweep :type Boolean) (SweepResult :type Hit%20Result%20Structure%20%28by%20ref%29))
  (Networking|SwitchHasAuthority
    (:Authority
      (bind _asbp_main_character_dong_jin (Utilities|Casting|CastToBP_MainCharacterDongJin OtherActor))
      (Variables|/Game/_DongJin/BP_MainCharacterDongJin.BP_MainCharacterDongJin_C|SetMaxAmmo _asbp_main_character_dong_jin (Utilities|Array|MakeArray (Utilities|Array|Get(acopy) (Variables|/Game/_DongJin/BP_MainCharacterDongJin.BP_MainCharacterDongJin_C|GetMaxAmmo _asbp_main_character_dong_jin)) (Utilities|Array|Get(acopy) (Variables|/Game/_DongJin/BP_MainCharacterDongJin.BP_MainCharacterDongJin_C|GetMaxAmmo _asbp_main_character_dong_jin) 1) (+ (Utilities|Array|Get(acopy) (Variables|/Game/_DongJin/BP_MainCharacterDongJin.BP_MainCharacterDongJin_C|GetMaxAmmo _asbp_main_character_dong_jin) 3) 5)))
      (bind _asbp_main_hud_dongjin (Utilities|Casting|CastToBP_MainHUD_Dongjin (HUD|GetHUD (Game|GetPlayerController 0))))
      (Default|SetAmmoUI _asbp_main_hud_dongjin)
      (Actor|DestroyActor))))

(fn ConstructionScript)