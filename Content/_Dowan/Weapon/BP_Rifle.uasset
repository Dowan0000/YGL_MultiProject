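; BP_Rifle is a rifle weapon Blueprint that shows a widget while the main character is within its overlap box.
; It extends the parent's box begin and end overlap events, calling the parent first, then casting to BP_MainCharacter to toggle the widget's visibility.
; Mesh custom depth toggles are present but disconnected, so they never run.
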(event EventBoxBeginOverlap
  (params (OverlappedComponent :type Primitive%20Component%20Object%20Reference) (OtherActor :type Actor%20Object%20Reference) (OtherComp :type Primitive%20Component%20Object%20Reference) (OtherBodyIndex :type Integer) (bFromSweep :type Boolean) (SweepResult :type Hit%20Result%20Structure%20%28by%20ref%29))
  (|CallParentFunction OverlappedComponent OtherActor OtherComp OtherBodyIndex bFromSweep SweepResult)
  (Utilities|Casting|CastToBP_MainCharacter OtherActor)
  (Rendering|SetVisibility (Variables|Default|GetWidget) true false))

(event EventBoxEndOverlap
  (params (OverlappedComponent :type Primitive%20Component%20Object%20Reference) (OtherActor :type Actor%20Object%20Reference) (OtherComp :type Primitive%20Component%20Object%20Reference) (OtherBodyIndex :type Integer))
  (|CallParentFunction OverlappedComponent OtherActor OtherComp OtherBodyIndex)
  (Utilities|Casting|CastToBP_MainCharacter OtherActor)
  (Rendering|SetVisibility (Variables|Default|GetWidget) false false))

(fn ConstructionScript)