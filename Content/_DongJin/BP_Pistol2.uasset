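; Pistol weapon Blueprint that extends a parent weapon with a pickup prompt, shot feedback and ammo tracking.
; Box overlap by a MainCharacter toggles a widget, and shooting calls the parent, prints a debug string and starts a camera shake.
; UseAmmo decrements a clamped count and reports whether a round was available.
; Ammo's RepNotify updates the HUD counter only when the owner is controlled by player controller 0.
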(event EventPressShoot
  (|CallParentFunction)
  (Development|PrintString "Hello")
  (CameraShakes|StartCameraShake (Variables|Default|GetCameraShakeSource) "/Game/_Dowan/Weapon/CameraShake/Pistol_CameraShake.Pistol_CameraShake_C" 1.0 "CameraLocal" "0, 0, 0"))

(event EventBoxBeginOverlap
  (params (OverlappedComponent :type Primitive%20Component%20Object%20Reference) (OtherActor :type Actor%20Object%20Reference) (OtherComp :type Primitive%20Component%20Object%20Reference) (OtherBodyIndex :type Integer) (bFromSweep :type Boolean) (SweepResult :type Hit%20Result%20Structure%20%28by%20ref%29))
  (|CallParentFunction OverlappedComponent OtherActor OtherComp OtherBodyIndex bFromSweep SweepResult)
  (Utilities|Casting|CastToMainCharacter OtherActor)
  (Rendering|SetVisibility (Variables|Default|GetWidget) true false))

(event EventBoxEndOverlap
  (params (OverlappedComponent :type Primitive%20Component%20Object%20Reference) (OtherActor :type Actor%20Object%20Reference) (OtherComp :type Primitive%20Component%20Object%20Reference) (OtherBodyIndex :type Integer))
  (|CallParentFunction OverlappedComponent OtherActor OtherComp OtherBodyIndex)
  (Utilities|Casting|CastToMainCharacter OtherActor)
  (Rendering|SetVisibility (Variables|Default|GetWidget) false false))

(fn ConstructionScript)

(fn UseAmmo
  (LocalVariables|SetCanUsed (> (Variables|Default|GetAmmo) 0))
  (Variables|Default|SetAmmo (Math|Integer|Clamp(Integer) (- (Variables|Default|GetAmmo) 1) 0 10))
  (return (LocalVariables|GetCanUsed)))

(fn UpdateAmmotoUI
  (params (Ammo :type Integer))
  (bind _returnvalue (Game|GetPlayerController 0))
  (bind _ownchar (Variables|Default|GetOwnChar))
  (Utilities|IsValid _ownchar
    (:Is%20Valid
      (if (== (Pawn|GetController _ownchar) _returnvalue)
        (bind _asbp_main_hud_dongjin (Utilities|Casting|CastToBP_MainHUD_Dongjin (HUD|GetHUD _returnvalue)))
        (Default|SetAmmo (Variables|/Game/_DongJin/BP_MainHUD_Dongjin.BP_MainHUD_Dongjin_C|GetWBP_AmmoCount _asbp_main_hud_dongjin) Ammo)))))

(fn OnRepAmmo
  (bind _ownchar (Variables|Default|GetOwnChar))
  (Utilities|IsValid _ownchar
    (:Is%20Valid
      (if (== (Pawn|GetController _ownchar) (Game|GetPlayerController 0))
        (CallFunction|UpdateAmmotoUI (Variables|Default|GetAmmo))))))