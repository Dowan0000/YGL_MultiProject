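; TCP chat client Blueprint that links the in-game chat widget to a socket server at a hardcoded localhost address.
; It connects on BeginPlay and stores the connection ID on connect, resetting it on disconnect.
; Received data is read as a string and passed through BP_MainHUD to its chat widget.
; SendMessage converts text to bytes and sends it over the stored connection.
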(event Custom|Disconnected
  (params (ConnectionId :type Integer))
  (Variables|Default|SetServerSocket -1))

(event Custom|Connected
  (params (ConnectionId :type Integer))
  (Variables|Default|SetServerSocket ConnectionId))

(event Custom|Message_Recd
  (params (ConnectionId :type Integer) (Message :type Array%20of%20Bytes))
  (bind _returnvalue (Class|TcpSocketConnection|MessageReadString Message (Utilities|Array|Length Message)))
  (bind _asbp_main_hud (Utilities|Casting|CastToBP_MainHUD (HUD|GetHUD (Game|GetPlayerController 0))))
  (Default|RecvMessage (Variables|/Game/_Dowan/UI/BP_MainHUD.BP_MainHUD_C|GetWBChatRef _asbp_main_hud) _returnvalue false))

(event EventBeginPlay
  (Class|TcpSocketConnection|Connect "127.0.0.1" 19934 (delegate Custom|Disconnected) (delegate Custom|Connected) (delegate Custom|Message_Recd)))

(fn ConstructionScript)

(fn SendMessage
  (params (Message :type String))
  (Class|TcpSocketConnection|SendData (Variables|Default|GetServerSocket) (Class|TcpSocketConnection|ToBytes(String) Message)))