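; Main HUD Blueprint that creates WBP_MainUI and drives its health, potion and weapon displays.
; Health starts from the character, then follows ShootingPlayerState's ChangeHp dispatcher, with BindPlayerState retrying on a timer until the cast succeeds.
; It also holds the potion count, gating use on remaining stock and updating the quick slot.
; SetWeaponUI re-fetches the widget from HUDWidget, rebinds health, passes the character to weapon slots and shows the equipped weapon's name.
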(event EventBeginPlay
  (bind _returnvalue (UserInterface|CreateWidget "/Game/_DongJin/Widget/WBP_MainUI.WBP_MainUI_C"))
  (bind _output_get (Variables|Default|SetWBP_MainUI _returnvalue))
  (bind _asbp_main_character_dong_jin (Utilities|Casting|CastToBP_MainCharacterDongJin (Game|GetPlayerCharacter 0)))
  (Default|SetHp _output_get (Variables|/Script/YGL_MultiProject.MainCharacter|GetHealth _asbp_main_character_dong_jin) (Variables|/Script/YGL_MultiProject.MainCharacter|GetMaxHealth _asbp_main_character_dong_jin))
  (UserInterface|Viewport|AddtoViewport _output_get 0)
  (CallFunction|BindPlayerState))

(event EventSetWeaponUI
  (CallFunction|WeaponUINameSet))

(fn ConstructionScript)

(fn UpdatePotion
  (bind _output_get (Variables|Default|SetPotion (+ (Variables|Default|GetPotion) 1)))
  (Default|SetPotion (Variables|/Game/_DongJin/Widget/WBP_MainUI.WBP_MainUI_C|GetWBP_QuickSlot (Variables|Default|GetWBP_MainUI)) _output_get))

(fn WeaponUI
  (bind _wbp_mainui (Variables|Default|GetWBP_MainUI))
  (bind _wbp_weaponslotinventroy (Variables|/Game/_DongJin/Widget/WBP_MainUI.WBP_MainUI_C|GetWBP_WeaponSlotInventroy _wbp_mainui))
  (Utilities|IsValid _wbp_weaponslotinventroy
    (:Is%20Valid
      (Utilities|FlowControl|Sequence
        (:then_0
          (Default|SetCharacter (Variables|/Game/_DongJin/Widget/WBP_WeaponSlotInventroy.WBP_WeaponSlotInventroy_C|GetWBP_WeaponSlot _wbp_weaponslotinventroy) (Variables|Default|GetCharacter)))
        (:then_1
          (Default|SetCharacter (Variables|/Game/_DongJin/Widget/WBP_WeaponSlotInventroy.WBP_WeaponSlotInventroy_C|GetWBP_WeaponSlot_0 _wbp_weaponslotinventroy) (Variables|Default|GetCharacter)))
        (:then_2
          (Default|SetCharacter (Variables|/Game/_DongJin/Widget/WBP_WeaponSlotInventroy.WBP_WeaponSlotInventroy_C|GetWBP_WeaponSlot_1 _wbp_weaponslotinventroy) (Variables|Default|GetCharacter)))))))

(fn OnRepPotion)

(fn UsePotion
  (if (CallFunction|IsCanUsePotion)
    (bind _output_get (Variables|Default|SetPotion (- (Variables|Default|GetPotion) 1)))
    (Default|SetPotion (Variables|/Game/_DongJin/Widget/WBP_MainUI.WBP_MainUI_C|GetWBP_QuickSlot (Variables|Default|GetWBP_MainUI)) _output_get)
    (return true)
    (else
      (return false))))

(fn IsCanUsePotion
  (return (> (Variables|Default|GetPotion) 0)))

(fn BindPlayerState
  (bind _asshooting_player_state (Utilities|Casting|CastToShootingPlayerState (Variables|/Script/Engine.Controller|GetPlayerState (Game|GetPlayerController 0)))
    (:then
      (EventDispatchers|BindEventtoEventDispatcherChangeHp _asshooting_player_state (EventDispatchers|CreateEvent :!event UpdateMyHp))
      (CallFunction|UpdateMyHp (Variables|/Game/_DongJin/ShootingPlayerState.ShootingPlayerState_C|GetCurHp _asshooting_player_state) (Variables|/Game/_DongJin/ShootingPlayerState.ShootingPlayerState_C|GetMaxHp _asshooting_player_state)))
    (:CastFailed
      (Utilities|Time|SetTimerbyFunctionName 0 "BindPlayerState" 0.1))))

(fn UpdateMyHp
  (params (CurHp :type Float%20%28single-precision%29) (MaxHp :type Float%20%28single-precision%29))
  (Default|SetHp (Variables|Default|GetWBP_MainUI) CurHp MaxHp))

(fn WeaponUINameSet
  (bind _character (Variables|Default|GetCharacter))
  (bind _equipweapon (Variables|/Script/YGL_MultiProject.MainCharacter|GetEquipWeapon _character))
  (bind _aswbp_main_ui (Utilities|Casting|CastToWBP_MainUI (Variables|Default|GetHUDWidget)))
  (Variables|Default|SetWBP_MainUI _aswbp_main_ui)
  (CallFunction|BindPlayerState)
  (Utilities|FlowControl|Sequence
    (:then_0
      (Default|SetCharacter (Variables|/Game/_DongJin/Widget/WBP_WeaponSlotInventroy.WBP_WeaponSlotInventroy_C|GetWBP_WeaponSlot (Variables|/Game/_DongJin/Widget/WBP_MainUI.WBP_MainUI_C|GetWBP_WeaponSlotInventroy (Variables|Default|GetWBP_MainUI))) (Variables|Default|GetCharacter)))
    (:then_1
      ;[1 1 1] 2번 Slot Update
      (Default|SetCharacter (Variables|/Game/_DongJin/Widget/WBP_WeaponSlotInventroy.WBP_WeaponSlotInventroy_C|GetWBP_WeaponSlot_0 (Variables|/Game/_DongJin/Widget/WBP_MainUI.WBP_MainUI_C|GetWBP_WeaponSlotInventroy (Variables|Default|GetWBP_MainUI))) (Variables|Default|GetCharacter)))
    (:then_2
      ;[1 1 1] 3번 Slot Update
      (Default|SetCharacter (Variables|/Game/_DongJin/Widget/WBP_WeaponSlotInventroy.WBP_WeaponSlotInventroy_C|GetWBP_WeaponSlot_1 (Variables|/Game/_DongJin/Widget/WBP_MainUI.WBP_MainUI_C|GetWBP_WeaponSlotInventroy (Variables|Default|GetWBP_MainUI))) (Variables|Default|GetCharacter)))
    (:then_3
      ;[1 1 1] 4번 Slot Update
      (Default|SetCharacter (Variables|/Game/_DongJin/Widget/WBP_WeaponSlotInventroy.WBP_WeaponSlotInventroy_C|GetWBP_WeaponSlot_2 (Variables|/Game/_DongJin/Widget/WBP_MainUI.WBP_MainUI_C|GetWBP_WeaponSlotInventroy (Variables|Default|GetWBP_MainUI))) (Variables|Default|GetCharacter)))
    (:then_4
      (Utilities|IsValid _equipweapon
        (:Is%20Valid
          ;[1 1 1] Weapon Name Update
          (Default|SetWeaponName (Variables|/Game/_DongJin/Widget/WBP_WeaponSlotInventroy.WBP_WeaponSlotInventroy_C|GetWBP_AmmoCount (Variables|/Game/_DongJin/Widget/WBP_MainUI.WBP_MainUI_C|GetWBP_WeaponSlotInventroy (Variables|Default|GetWBP_MainUI))) (Utilities|Text|ToText(Name) (Variables|/Script/YGL_MultiProject.WeaponBase|GetRowName _equipweapon))))))))