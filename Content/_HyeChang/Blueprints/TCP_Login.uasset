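; TCP login client that talks to a hard-coded login server and drives the game's login flow.
; It connects on BeginPlay, tracks the socket ID, and sends text through SendMessage, disconnecting if a send fails.
; String replies show timed success, already-logged-in or unknown-ID widgets; success then opens the session-finding level as a listen server.
; Any other reply is saved as the player name in ShootingGameInstance.
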(event Custom|Disconnected
  (params (ConnectionId :type Integer))
  (Variables|Default|SetServerSocket -1))

(event Custom|Connected
  (params (ConnectionId :type Integer))
  (Variables|Default|SetServerSocket ConnectionId))

(event Custom|Message_Recd
  (params (ConnectionId :type Integer) (Message :type Array%20of%20Bytes))
  (bind _returnvalue (Class|TcpSocketConnection|MessageReadString Message (Utilities|Array|Length Message)))
  (if (Utilities|Enum|Equal(Enum) _returnvalue "LoginSuccess")
    (Development|PrintString "로그인 성공 !")
    (bind _returnvalue_2 (UserInterface|CreateWidget "/Game/_HyeChang/Widgets/LoginSuccessWidget.LoginSuccessWidget_C"))
    (UserInterface|Viewport|AddtoViewport _returnvalue_2 0)
    (Utilities|FlowControl|Delay 2.0)
    (Widget|RemovefromParent _returnvalue_2)
    (Game|OpenLevel(byName) "FIndSessionLevel" false "listen")
    (elif (Utilities|Enum|Equal(Enum) _returnvalue "Already_Accpet")
      (Development|PrintString "이미 접속중인 아이디입니다.")
      (bind _returnvalue_3 (UserInterface|CreateWidget "/Game/_HyeChang/Widgets/LoginFailWidget.LoginFailWidget_C"))
      (UserInterface|Viewport|AddtoViewport _returnvalue_3 0)
      (Utilities|FlowControl|Delay 2.0)
      (Widget|RemovefromParent _returnvalue_3)
      (elif (Utilities|Enum|Equal(Enum) _returnvalue "Not_Exits")
        (Development|PrintString "존재하지않는 아이디입니다.")
        (bind _returnvalue_4 (UserInterface|CreateWidget "/Game/_HyeChang/Widgets/NotExitsLoginWidget.NotExitsLoginWidget_C"))
        (UserInterface|Viewport|AddtoViewport _returnvalue_4 0)
        (Utilities|FlowControl|Delay 2.0)
        (Widget|RemovefromParent _returnvalue_4)
        (else
          (bind _output_get (Variables|Default|SetLoginPlayerName _returnvalue))
          (bind _asshooting_game_instance (Utilities|Casting|CastToShootingGameInstance (Game|GetGameInstance)))
          (Default|SetPlayerName _asshooting_game_instance _output_get))))))

(event EventBeginPlay
  (Class|TcpSocketConnection|Connect "172.16.2.84" 19936 (delegate Custom|Disconnected) (delegate Custom|Connected) (delegate Custom|Message_Recd)))

(fn ConstructionScript)

(fn SendMessage
  (params (Message :type String))
  (bind _returnvalue (Class|TcpSocketConnection|SendData (Variables|Default|GetServerSocket) (Class|TcpSocketConnection|ToBytes(String) Message)))
  (if (not _returnvalue)
    (Class|TcpSocketConnection|Disconnect (Variables|Default|GetServerSocket))
    (Variables|Default|SetServerSocket 0)))