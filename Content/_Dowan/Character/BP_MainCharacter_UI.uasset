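; BP_MainCharacter_UI is a character Blueprint meant to set up the main HUD and its weapon slots, but none of that logic is connected.
; BeginPlay and the SetWeaponUI event are both empty.
; Disconnected nodes would call the parent BeginPlay, add a WBP_MainUIoo widget to the viewport, and pass the character to three slots in its weapon slot inventory.
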(event EventBeginPlay)

(event EventSetWeaponUI)

(fn ConstructionScript)