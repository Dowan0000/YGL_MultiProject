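; BP_PistolAmmo is an ammo pickup that tops up a character's pistol reserve.
; On box overlap, the server casts the other actor to BP_MainCharacterDongJin and checks whether it has a pistol.
; If so, it adds a fixed amount to the first inventory slot's MaxAmmo, clamped to a cap, then destroys itself.
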(event OnComponentBeginOverlap(Box)
  (params (OverlappedComponent :type Primitive%20Component%20Object%20Reference) (OtherActor :type Actor%20Object%20Reference) (OtherComp :type Primitive%20Component%20Object%20Reference) (OtherBodyIndex :type Integer) (bFromSweep :type Boolean) (SweepResult :type Hit%20Result%20Structure%20%28by%20ref%29))
  (Networking|SwitchHasAuthority
    (:Authority
      (bind _asbp_main_character_dong_jin (Utilities|Casting|CastToBP_MainCharacterDongJin OtherActor))
      (if (Variables|/Script/YGL_MultiProject.MainCharacter|GetHasPistol _asbp_main_character_dong_jin)
        (Variables|/Script/YGL_MultiProject.WeaponBase|SetMaxAmmo (Utilities|Array|Get(acopy) (Variables|/Script/YGL_MultiProject.MainCharacter|GetInventory _asbp_main_character_dong_jin)) (Math|Integer|Clamp(Integer) (+ (Variables|/Script/YGL_MultiProject.WeaponBase|GetMaxAmmo (Utilities|Array|Get(acopy) (Variables|/Script/YGL_MultiProject.MainCharacter|GetInventory _asbp_main_character_dong_jin))) 10) 0 30))
        (Actor|DestroyActor)))))

(fn ConstructionScript)