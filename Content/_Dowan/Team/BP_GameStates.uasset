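; Team match game-state Blueprint that shows the end-of-match win, lose or draw screen to local players.
; The OnRep handler for STGameState dispatches to Team A win, Team B win, or TimeOver, which results in a draw.
; Each screen function loops both team controller arrays, acting only on local controllers: it adds the result widget, hides HUD and chat, switches to UI-only input and nearly stops movement.
; Winners, and both teams on draws, also trigger team ending calls.
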(event EventBeginPlay)

(event EventTick
  (params (DeltaSeconds :type Float%20%28single-precision%29)))

(fn ConstructionScript)

(fn TeamAWinScreen
  (bind _returnvalue (Game|GetPlayerController 0))
  (bind _returnvalue_2 (Game|GetPlayerController 0))
  (Utilities|FlowControl|Sequence
    (:then_0
      (for _array_element (Variables|Default|GetTeamAController)
        (Utilities|IsValid _array_element
          (:Is%20Valid
            (if (Pawn|IsLocalController _array_element)
              (bind _asteam_player_controller (Utilities|Casting|CastToTeamPlayerController _array_element))
              (Default|TeamAEnding _asteam_player_controller)
              (bind _returnvalue_3 (UserInterface|CreateWidget "/Game/_Dowan/UI/WBP_ScreenWin.WBP_ScreenWin_C" _array_element))
              (UserInterface|Viewport|AddtoViewport _returnvalue_3 0)
              (bind _asbp_main_hud (Utilities|Casting|CastToBP_MainHUD (HUD|GetHUD (Game|GetPlayerController 0))))
              (Input|SetInputModeUIOnly _returnvalue (Variables|/Game/_Dowan/UI/BP_MainHUD.BP_MainHUD_C|GetWBP_MainUI _asbp_main_hud) "DoNotLock")
              (Variables|/Script/Engine.PlayerController|SetbShowMouseCursor _returnvalue true)
              (Widget|SetVisibility (Variables|/Game/_Dowan/UI/BP_MainHUD.BP_MainHUD_C|GetWBChatRef _asbp_main_hud) "Hidden")
              (Variables|/Script/Engine.CharacterMovementComponent|SetMaxWalkSpeed (Variables|/Script/Engine.Character|GetCharacterMovement (Game|GetPlayerCharacter 0)) 1.0))))))
    (:then_1
      (for _array_element_2 (Variables|Default|GetTeamBController)
        (Utilities|IsValid _array_element_2
          (:Is%20Valid
            (if (Pawn|IsLocalController _array_element_2)
              (bind _returnvalue_4 (UserInterface|CreateWidget "/Game/_Dowan/UI/WBP_ScreenLose.WBP_ScreenLose_C" _array_element_2))
              (UserInterface|Viewport|AddtoViewport _returnvalue_4 0)
              (bind _asbp_main_hud_2 (Utilities|Casting|CastToBP_MainHUD (HUD|GetHUD (Game|GetPlayerController 0))))
              (Input|SetInputModeUIOnly _returnvalue_2 (Variables|/Game/_Dowan/UI/BP_MainHUD.BP_MainHUD_C|GetWBP_MainUI _asbp_main_hud_2) "DoNotLock")
              (Variables|/Script/Engine.PlayerController|SetbShowMouseCursor _returnvalue_2 true)
              (Widget|SetVisibility (Variables|/Game/_Dowan/UI/BP_MainHUD.BP_MainHUD_C|GetWBChatRef _asbp_main_hud_2) "Hidden")
              (Variables|/Script/Engine.CharacterMovementComponent|SetMaxWalkSpeed (Variables|/Script/Engine.Character|GetCharacterMovement (Game|GetPlayerCharacter 0)) 1.0))))))))

(fn TeamBWinScreen
  (bind _returnvalue (Game|GetPlayerController 0))
  (bind _returnvalue_2 (Game|GetPlayerController 0))
  (Utilities|FlowControl|Sequence
    (:then_0
      (for _array_element (Variables|Default|GetTeamAController)
        (Utilities|IsValid _array_element
          (:Is%20Valid
            (if (Pawn|IsLocalController _array_element)
              (bind _returnvalue_3 (UserInterface|CreateWidget "/Game/_Dowan/UI/WBP_ScreenLose.WBP_ScreenLose_C" _array_element))
              (UserInterface|Viewport|AddtoViewport _returnvalue_3 0)
              (bind _asbp_main_hud (Utilities|Casting|CastToBP_MainHUD (HUD|GetHUD (Game|GetPlayerController 0))))
              (Input|SetInputModeUIOnly _returnvalue (Variables|/Game/_Dowan/UI/BP_MainHUD.BP_MainHUD_C|GetWBP_MainUI _asbp_main_hud) "DoNotLock")
              (Variables|/Script/Engine.PlayerController|SetbShowMouseCursor _returnvalue true)
              (Widget|SetVisibility (Variables|/Game/_Dowan/UI/BP_MainHUD.BP_MainHUD_C|GetWBChatRef _asbp_main_hud) "Hidden")
              (Variables|/Script/Engine.CharacterMovementComponent|SetMaxWalkSpeed (Variables|/Script/Engine.Character|GetCharacterMovement (Game|GetPlayerCharacter 0)) 1.0))))))
    (:then_1
      (for _array_element_2 (Variables|Default|GetTeamBController)
        (Utilities|IsValid _array_element_2
          (:Is%20Valid
            (if (Pawn|IsLocalController _array_element_2)
              (bind _asteam_player_controller (Utilities|Casting|CastToTeamPlayerController _array_element_2))
              (Default|TeamBEnding _asteam_player_controller)
              (bind _returnvalue_4 (UserInterface|CreateWidget "/Game/_Dowan/UI/WBP_ScreenWin.WBP_ScreenWin_C" _array_element_2))
              (UserInterface|Viewport|AddtoViewport _returnvalue_4 0)
              (bind _asbp_main_hud_2 (Utilities|Casting|CastToBP_MainHUD (HUD|GetHUD (Game|GetPlayerController 0))))
              (Input|SetInputModeUIOnly _returnvalue_2 0 "DoNotLock")
              (Variables|/Script/Engine.PlayerController|SetbShowMouseCursor _returnvalue_2 true)
              (Widget|SetVisibility (Variables|/Game/_Dowan/UI/BP_MainHUD.BP_MainHUD_C|GetWBChatRef _asbp_main_hud_2) "Hidden")
              (Variables|/Script/Engine.CharacterMovementComponent|SetMaxWalkSpeed (Variables|/Script/Engine.Character|GetCharacterMovement (Game|GetPlayerCharacter 0)) 1.0))))))))

(fn OnRepSTGameState
  (Utilities|FlowControl|Sequence
    (:then_0
      (if (Utilities|Enum|Equal(Enum) (Variables|Default|GetST_GameState) "NewEnumerator2")
        (CallFunction|TeamAWinScreen)))
    (:then_1
      (if (Utilities|Enum|Equal(Enum) (Variables|Default|GetST_GameState) "NewEnumerator3")
        (CallFunction|TeamBWinScreen)))
    (:then_2
      (if (Utilities|Enum|Equal(Enum) (Variables|Default|GetST_GameState) "NewEnumerator4")
        (CallFunction|TimeOver)))))

(fn TimeOver
  (CallFunction|TeamDrawScreen))

(fn TeamDrawScreen
  (bind _returnvalue (Game|GetPlayerController 0))
  (bind _returnvalue_2 (Game|GetPlayerController 0))
  (Utilities|FlowControl|Sequence
    (:then_0
      (for _array_element (Variables|Default|GetTeamAController)
        (Utilities|IsValid _array_element
          (:Is%20Valid
            (if (Pawn|IsLocalController _array_element)
              (bind _asteam_player_controller (Utilities|Casting|CastToTeamPlayerController _array_element))
              (Default|TeamAEnding _asteam_player_controller)
              (bind _returnvalue_3 (UserInterface|CreateWidget "/Game/_Dowan/UI/WBP_ScreenDraw.WBP_ScreenDraw_C" _array_element))
              (UserInterface|Viewport|AddtoViewport _returnvalue_3 0)
              (bind _asbp_main_hud (Utilities|Casting|CastToBP_MainHUD (HUD|GetHUD (Game|GetPlayerController 0))))
              (Input|SetInputModeUIOnly _returnvalue 0 "DoNotLock")
              (Variables|/Script/Engine.PlayerController|SetbShowMouseCursor _returnvalue true)
              (Widget|SetVisibility (Variables|/Game/_Dowan/UI/BP_MainHUD.BP_MainHUD_C|GetWBChatRef _asbp_main_hud) "Hidden")
              (Variables|/Script/Engine.CharacterMovementComponent|SetMaxWalkSpeed (Variables|/Script/Engine.Character|GetCharacterMovement (Game|GetPlayerCharacter 0)) 1.0))))))
    (:then_1
      (for _array_element_2 (Variables|Default|GetTeamBController)
        (Utilities|IsValid _array_element_2
          (:Is%20Valid
            (if (Pawn|IsLocalController _array_element_2)
              (bind _asteam_player_controller_2 (Utilities|Casting|CastToTeamPlayerController _array_element_2))
              (Default|TeamBEnding _asteam_player_controller_2)
              (bind _returnvalue_4 (UserInterface|CreateWidget "/Game/_Dowan/UI/WBP_ScreenDraw.WBP_ScreenDraw_C" _array_element_2))
              (UserInterface|Viewport|AddtoViewport _returnvalue_4 0)
              (bind _asbp_main_hud_2 (Utilities|Casting|CastToBP_MainHUD (HUD|GetHUD (Game|GetPlayerController 0))))
              (Input|SetInputModeUIOnly _returnvalue_2 0 "DoNotLock")
              (Variables|/Script/Engine.PlayerController|SetbShowMouseCursor _returnvalue_2 true)
              (Widget|SetVisibility (Variables|/Game/_Dowan/UI/BP_MainHUD.BP_MainHUD_C|GetWBChatRef _asbp_main_hud_2) "Hidden")
              (Variables|/Script/Engine.CharacterMovementComponent|SetMaxWalkSpeed (Variables|/Script/Engine.Character|GetCharacterMovement (Game|GetPlayerCharacter 0)) 1.0))))))))