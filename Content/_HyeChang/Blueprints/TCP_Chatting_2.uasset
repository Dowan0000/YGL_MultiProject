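; TCP chat client that links the game to a chat server at a hardcoded IP and port, connecting on BeginPlay.
; Connection callbacks store or clear the server socket ID.
; Incoming bytes are decoded to a string and passed to the LobbyHud chat widget.
; SendMessage converts text to bytes and sends it; its disconnect branch tests a constant true, so it never runs.
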(event Custom|Disconnected
  (params (ConnectionId :type Integer))
  (Variables|Default|SetServerSocket -1))

(event Custom|Connected
  (params (ConnectionId :type Integer))
  (Variables|Default|SetServerSocket ConnectionId))

(event Custom|Message_Recd
  (params (ConnectionId :type Integer) (Message :type Array%20of%20Bytes))
  (bind _returnvalue (Class|TcpSocketConnection|MessageReadString Message (Utilities|Array|Length Message)))
  (bind _aslobby_hud (Utilities|Casting|CastToLobbyHud (HUD|GetHUD (Game|GetPlayerController 0))))
  (Default|RecvMessage (Variables|/Game/_HyeChang/GameMode/LobbyHud.LobbyHud_C|GetWB_Chat%20 _aslobby_hud) _returnvalue false))

(event EventBeginPlay
  (Class|TcpSocketConnection|Connect "172.16.2.84" 19934 (delegate Custom|Disconnected) (delegate Custom|Connected) (delegate Custom|Message_Recd)))

(fn ConstructionScript)

(fn SendMessage
  (params (Message :type String))
  (Class|TcpSocketConnection|SendData (Variables|Default|GetServerSocket) (Class|TcpSocketConnection|ToBytes(String) Message))
  (if (not true)
    (Class|TcpSocketConnection|Disconnect (Variables|Default|GetServerSocket))
    (Variables|Default|SetServerSocket 0)))