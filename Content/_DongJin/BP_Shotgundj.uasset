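; BP_Shotgundj is a shotgun weapon that extends a parent weapon class with an ammo limit, a proximity widget and camera shake.
; Box overlap events run the parent logic, then show or hide the widget as a MainCharacter enters or leaves.
; PressShoot calls the parent shot only while ammo remains, then decrements it through UseAmmo.
; CameraShake plays the sniper's shake asset only for a locally controlled character.
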(event EventPressShoot
  (if (> (Variables|Default|GetCurAmmo) 0)
    (|CallParentFunction)
    (CallFunction|UseAmmo)))

(event EventCameraShake
  (if (Pawn|IsLocallyControlled (Variables|Default|GetCharacter))
    (CameraShakes|StartCameraShake (Variables|Default|GetCameraShakeSource) "/Game/_Dowan/Weapon/CameraShake/Sniper_CameraShake.Sniper_CameraShake_C" 1.0 "CameraLocal" "0, 0, 0")))

(event EventBoxBeginOverlap
  (params (OverlappedComponent :type Primitive%20Component%20Object%20Reference) (OtherActor :type Actor%20Object%20Reference) (OtherComp :type Primitive%20Component%20Object%20Reference) (OtherBodyIndex :type Integer) (bFromSweep :type Boolean) (SweepResult :type Hit%20Result%20Structure%20%28by%20ref%29))
  (|CallParentFunction OverlappedComponent OtherActor OtherComp OtherBodyIndex bFromSweep SweepResult)
  (Utilities|Casting|CastToMainCharacter OtherActor)
  (Rendering|SetVisibility (Variables|Default|GetWidget) true false))

(event EventBoxEndOverlap
  (params (OverlappedComponent :type Primitive%20Component%20Object%20Reference) (OtherActor :type Actor%20Object%20Reference) (OtherComp :type Primitive%20Component%20Object%20Reference) (OtherBodyIndex :type Integer))
  (|CallParentFunction OverlappedComponent OtherActor OtherComp OtherBodyIndex)
  (Utilities|Casting|CastToMainCharacter OtherActor)
  (Rendering|SetVisibility (Variables|Default|GetWidget) false false))

(fn ConstructionScript)

(fn UseAmmo
  (Variables|Default|SetCurAmmo (- (Variables|Default|GetCurAmmo) 1))
  (return))