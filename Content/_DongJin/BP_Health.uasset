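; BP_Health is a health potion pickup that the two main character Blueprints can collect.
; When its Sphere begins overlapping an actor, it tries a cast to BP_MainCharacter_A1 and to BP_MainCharacter_B1 in sequence.
; If the matching character holds zero potions, it increments that character's Potion count and destroys itself, so a character already carrying one leaves the pickup in place.
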(event OnComponentBeginOverlap(Sphere)
  (params (OverlappedComponent :type Primitive%20Component%20Object%20Reference) (OtherActor :type Actor%20Object%20Reference) (OtherComp :type Primitive%20Component%20Object%20Reference) (OtherBodyIndex :type Integer) (bFromSweep :type Boolean) (SweepResult :type Hit%20Result%20Structure%20%28by%20ref%29))
  (Utilities|FlowControl|Sequence
    (:then_0
      (bind _asbp_main_character_a1 (Utilities|Casting|CastToBP_MainCharacter_A1 OtherActor))
      (if (== (Variables|/Game/_DongJin/12_24/TeamACharDongjin/BP_MainCharacter_A1.BP_MainCharacter_A1_C|GetPotion _asbp_main_character_a1) 0)
        (Variables|/Game/_DongJin/12_24/TeamACharDongjin/BP_MainCharacter_A1.BP_MainCharacter_A1_C|SetPotion _asbp_main_character_a1 (+ (Variables|/Game/_DongJin/12_24/TeamACharDongjin/BP_MainCharacter_A1.BP_MainCharacter_A1_C|GetPotion _asbp_main_character_a1) 1))
        (Actor|DestroyActor)))
    (:then_1
      (bind _asbp_main_character_b1 (Utilities|Casting|CastToBP_MainCharacter_B1 OtherActor))
      (if (== (Variables|/Game/_DongJin/12_24/TeamBCharDongjin/BP_MainCharacter_B1.BP_MainCharacter_B1_C|GetPotion _asbp_main_character_b1) 0)
        (Variables|/Game/_DongJin/12_24/TeamBCharDongjin/BP_MainCharacter_B1.BP_MainCharacter_B1_C|SetPotion _asbp_main_character_b1 (+ (Variables|/Game/_DongJin/12_24/TeamBCharDongjin/BP_MainCharacter_B1.BP_MainCharacter_B1_C|GetPotion _asbp_main_character_b1) 1))
        (Actor|DestroyActor)))))

(fn ConstructionScript)