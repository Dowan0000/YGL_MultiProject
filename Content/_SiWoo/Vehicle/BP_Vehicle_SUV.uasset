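; BP_Vehicle_SUV is a drivable SUV that the player character can enter and exit.
; Axis and handbrake inputs feed the VehicleMovement component and controller camera rotation.
; OnInteracted stores the character, disables its capsule collision, hands possession to the SUV and hides its mesh.
; ExitVehicle restores collision, possession and visibility, teleporting the character to a mostly world-space offset from the vehicle.
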(event EventOnInteracted
  (params (InPlayer :type BP%20Main%20Character%20SW%20Object%20Reference))
  (Variables|Default|SetBP_MainCharacter_SW InPlayer)
  (Collision|SetCollisionEnabled (Variables|/Script/Engine.Character|GetCapsuleComponent (Variables|Default|GetBP_MainCharacter_SW)) "NoCollision")
  (Pawn|Possess (Pawn|GetController (Variables|Default|GetBP_MainCharacter_SW)) self)
  (Rendering|SetVisibility (Variables|/Script/Engine.Character|GetMesh (Variables|Default|GetBP_MainCharacter_SW)) false true))

(event Input|ActionEvents|InputActionHandBreak
  (params (Key :type Key%20Structure :default "None"))
  (:Pressed
    (Class|WheeledVehicleMovementComponent|SetHandbrakeInput (Variables|Default|GetVehicleMovement) true))
  (:Released
    (Class|WheeledVehicleMovementComponent|SetHandbrakeInput (Variables|Default|GetVehicleMovement) false)))

(event Input|ActionEvents|InputActionExitVehicle
  (params (Key :type Key%20Structure :default "None"))
  (bind _bp_maincharacter_sw (Variables|Default|GetBP_MainCharacter_SW))
  (:Pressed
    (bind _bp_maincharacter_sw_2 (Variables|Default|GetBP_MainCharacter_SW)
      (:then
        (Collision|SetCollisionEnabled (Variables|/Script/Engine.Character|GetCapsuleComponent _bp_maincharacter_sw_2) "QueryAndPhysics")
        (Pawn|Possess (Pawn|GetController) _bp_maincharacter_sw)
        (Transformation|SetActorLocation _bp_maincharacter_sw (+ (Transformation|GetActorLocation) "100.000000,-200.000000, 0" (Transformation|GetActorForwardVector)) false true)
        (Rendering|SetVisibility (Variables|/Script/Engine.Actor|GetRootComponent _bp_maincharacter_sw) true true))
      (:else))))

(event Input|AxisEvents|InputAxisMoveForward
  (params (AxisValue :type Float%20%28single-precision%29))
  (Class|WheeledVehicleMovementComponent|SetThrottleInput (Variables|Default|GetVehicleMovement) AxisValue))

(event Input|AxisEvents|InputAxisMoveRight
  (params (AxisValue :type Float%20%28single-precision%29))
  (Class|WheeledVehicleMovementComponent|SetSteeringInput (Variables|Default|GetVehicleMovement) AxisValue))

(event Input|AxisEvents|InputAxisLookUp
  (params (AxisValue :type Float%20%28single-precision%29))
  (Pawn|Input|AddControllerPitchInput AxisValue))

(event Input|AxisEvents|InputAxisTurn
  (params (AxisValue :type Float%20%28single-precision%29))
  (Pawn|Input|AddControllerYawInput AxisValue))

(fn ConstructionScript)