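; Drivable SUV vehicle pawn that feeds throttle, steering and handbrake input to its vehicle movement component, with mouse-look axes for the controller.
; ExitVehicle runs ReqExit into ResExit, which repossesses the stored PlayerCharacter, teleports it beside the car, unhides and detaches it, and frees the driver seat.
; OnInteracted is empty: the authority-checked boarding logic for a possessing driver and an attached second passenger is disconnected and never runs.
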(event Custom|ReqExit
  (CallFunction|ResExit))

(event Custom|ResExit
  (Utilities|IsValid (Variables|Default|GetPlayerCharacter)
    (:Is%20Valid
      (Collision|SetActorEnableCollision (Variables|Default|GetPlayerCharacter) true)
      (bind _asplayer_controller (Utilities|Casting|CastToPlayerController (Pawn|GetController)))
      (Pawn|Possess _asplayer_controller (Variables|Default|GetPlayerCharacter))
      (Transformation|SetActorLocation (Variables|Default|GetPlayerCharacter) (+ (Transformation|GetActorLocation) "100.000000,-200.000000,100.000000") false true)
      (Rendering|SetActorHiddenInGame (Variables|Default|GetPlayerCharacter) false)
      (Transformation|DetachFromActor (Variables|Default|GetPlayerCharacter) "KeepWorld" "KeepWorld" "KeepWorld")
      (Variables|Default|SetPlayerCharacter 0)
      (Variables|Default|SetSeat1 false))))

(event EventOnInteracted
  (params (InPlayer :type BP%20Main%20Character%20SW%20Object%20Reference)))

(event Input|ActionEvents|InputActionHandBreak
  (params (Key :type Key%20Structure :default "None"))
  (:Pressed
    (Class|WheeledVehicleMovementComponent|SetHandbrakeInput (Variables|Default|GetVehicleMovement) true))
  (:Released
    (Class|WheeledVehicleMovementComponent|SetHandbrakeInput (Variables|Default|GetVehicleMovement) false)))

(event Input|ActionEvents|InputActionExitVehicle
  (params (Key :type Key%20Structure :default "None"))
  (:Pressed
    (CallFunction|ReqExit)))

(event Input|AxisEvents|InputAxisMoveForward
  (params (AxisValue :type Float%20%28single-precision%29))
  (Class|WheeledVehicleMovementComponent|SetThrottleInput (Variables|Default|GetVehicleMovement) AxisValue))

(event Input|AxisEvents|InputAxisMoveRight
  (params (AxisValue :type Float%20%28single-precision%29))
  (Class|WheeledVehicleMovementComponent|SetSteeringInput (Variables|Default|GetVehicleMovement) AxisValue))

(event Input|AxisEvents|InputAxisLookUp
  (params (AxisValue :type Float%20%28single-precision%29))
  (Pawn|Input|AddControllerPitchInput AxisValue))

(event Input|AxisEvents|InputAxisTurn
  (params (AxisValue :type Float%20%28single-precision%29))
  (Pawn|Input|AddControllerYawInput AxisValue))

(fn ConstructionScript)