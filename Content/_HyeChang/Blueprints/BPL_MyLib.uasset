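; Blueprint function library of text validation checks, with helpers named for ID/password and player name input.
; Each returns a boolean from a character-length cap, with a separate limit per use.
; The general and ID/password checks also require a substring search to find nothing, though its search string appears empty.
; The full text check adds a non-empty test on top of the lite version.
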(fn MyLibCheckText
  (params (InputPin :type Text))
  (return (and (Utilities|Enum|NotEqual(Enum) InputPin (Utilities|Text|MakeLiteralText "")) (CallFunction|MyLibCheckTextLite InputPin))))

(fn MyLibCheckTextLite
  (params (InputPin :type Text))
  (bind _returnvalue (Utilities|String|ToString(Text) InputPin))
  (return (and (< (Utilities|String|Len _returnvalue) 12) (== (Utilities|String|FindSubstring _returnvalue " ") -1))))

(fn Id&PwdCount
  (params (InText :type Text))
  (bind _returnvalue (Utilities|String|ToString(Text) InText))
  (return (and (< (Utilities|String|Len _returnvalue) 20) (== (Utilities|String|FindSubstring _returnvalue " ") -1))))

(fn PlayerNameCount
  (params (InText :type Text))
  (return (< (Utilities|String|Len (Utilities|String|ToString(Text) InText)) 10)))