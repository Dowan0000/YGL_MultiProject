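; Player character Blueprint that adds vehicle boarding, chat focus, potion healing and weapon reloading, wired to the main HUD.
; Capsule overlap caches a nearby SUV, which ExitVehicle boards through interface messages or exits by detaching.
; Potion, reload and boarding inputs pass through paired request/response events, with OnRep_Potion refreshing the HUD.
; Reload plays a weapon-type montage, while ReloadAmmo runs per-weapon functions whose casts select the matching magazine math.
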(event OnComponentBeginOverlap(CapsuleComponent)
  (params (OverlappedComponent :type Primitive%20Component%20Object%20Reference) (OtherActor :type Actor%20Object%20Reference) (OtherComp :type Primitive%20Component%20Object%20Reference) (OtherBodyIndex :type Integer) (bFromSweep :type Boolean) (SweepResult :type Hit%20Result%20Structure%20%28by%20ref%29))
  (if (Utilities|DoesObjectImplementInterface OtherActor "/Game/_Dowan/Vehicle/BPI_Interaction2.BPI_Interaction2_C")
    (bind _asbp_vehicle_suv (Utilities|Casting|CastToBP_Vehicle_SUV OtherActor))
    (Variables|Default|SetAs%20BP%20Vehicle%20SUV _asbp_vehicle_suv)
    (Variables|Default|SetVehicletest true)))

(event OnComponentEndOverlap(CapsuleComponent)
  (params (OverlappedComponent :type Primitive%20Component%20Object%20Reference) (OtherActor :type Actor%20Object%20Reference) (OtherComp :type Primitive%20Component%20Object%20Reference) (OtherBodyIndex :type Integer))
  (if (Utilities|DoesObjectImplementInterface OtherActor "/Game/_Dowan/Vehicle/BPI_Interaction2.BPI_Interaction2_C")
    (Variables|Default|SetAs%20BP%20Vehicle%20SUV 0)
    (Variables|Default|SetVehicletest false)))

(event Custom|VehicleMul
  (Class|BPIInteraction2|OnInteracted(Message) (stale OnComponentBeginOverlap(CapsuleComponent) OtherActor) self))

(event Custom|VehicleServer
  (CallFunction|VehicleMul))

(event Custom|ReqReload
  ;[1 1 1] Reload
  (CallFunction|ResReload))

(event Custom|ResReload
  ;[1 1 1] Reload
  (switch Utilities|FlowControl|Switch|SwitchonEItemType (Variables|/Script/YGL_MultiProject.WeaponBase|GetItemType (Variables|Default|GetEquipWeapon))
    (:EIT_Pistol
      (Animation|PlayAnimMontage "/Game/_DongJin/12_24/TeamBCharDongjin/TeamBAnim/ReloadPistol.ReloadPistol" 1.0 "None"))
    (:EIT_Rifle
      (Animation|PlayAnimMontage "/Game/_DongJin/12_24/TeamBCharDongjin/TeamBAnim/ReloadRifle.ReloadRifle" 1.0 "None" :!label _label))
    (:EIT_Sniper
      (goto _label))
    (:EIT_Launcher
      (goto _label))))

(event Custom|ReqUsePotion
  ;[1 1 1] potion use & heal
  (CallFunction|ResUsePotion))

(event Custom|ResUsePotion
  ;[1 1 1] potion use & heal
  (if (> (Variables|Default|GetPotion) 0)
    (Variables|Default|SetPotion (- (Variables|Default|GetPotion) 1))
    (Variables|Default|SetHealth (+ (Variables|Default|GetHealth) 5e+01))
    (CallFunction|UsePotiononCli)))

(event Custom|UsePotionOnCli
  ;[1 1 1] potion use & heal
  (Default|SetHealth (Variables|/Game/_Dowan/UI/BP_MainHUD.BP_MainHUD_C|GetWBP_MainUI (Variables|Default|GetMain%20HUD)) (/ (Variables|Default|GetHealth) (Variables|Default|GetMaxHealth))))

(event EventBeginPlay
  (Utilities|FlowControl|Delay 2.0)
  (|CallParentFunction)
  (bind _asbp_main_hud (Utilities|Casting|CastToBP_MainHUD (HUD|GetHUD (Game|GetPlayerController 0))))
  (bind _output_get (Variables|Default|SetMain%20HUD _asbp_main_hud))
  (Default|SetCharacterB (Variables|/Game/_DongJin/Widget/WBP_WeaponSlotInventroy.WBP_WeaponSlotInventroy_C|GetWBP_AmmoCount (Variables|/Game/_DongJin/Widget/WBP_MainUIoo.WBP_MainUIoo_C|GetWBP_WeaponSlotInventroy (Variables|/Game/_Dowan/UI/BP_MainHUD.BP_MainHUD_C|GetWBP_MainUI _output_get))) self))

(event Input|ActionEvents|InputActionUsePotion
  (params (Key :type Key%20Structure :default "None"))
  ;[1 1 1] potion use & heal
  (:Pressed
    (CallFunction|ReqUsePotion)))

(event Input|ActionEvents|InputActionReload
  (params (Key :type Key%20Structure :default "None"))
  ;[1 1 1] Reload
  (:Pressed
    (CallFunction|ReqReload)))

(event Input|ActionEvents|InputActionChattingEnter
  (params (Key :type Key%20Structure :default "None"))
  (:Pressed
    (bind _asbp_main_hud (Utilities|Casting|CastToBP_MainHUD (HUD|GetHUD (Game|GetPlayerController 0))))
    (if (not (Class|Widget|HasKeyboardFocus (Variables|/Game/_HyeChang/Widgets/WB_Chat.WB_Chat_C|GetChatMessage_InputBox (Variables|/Game/_Dowan/UI/BP_MainHUD.BP_MainHUD_C|GetWBChatRef _asbp_main_hud))))
      (Input|SetInputModeUIOnly (Game|GetPlayerController 0) (Variables|/Game/_HyeChang/Widgets/WB_Chat.WB_Chat_C|GetChatMessage_InputBox (Variables|/Game/_Dowan/UI/BP_MainHUD.BP_MainHUD_C|GetWBChatRef _asbp_main_hud)) "DoNotLock"))))

(event Input|ActionEvents|InputActionExitVehicle
  (params (Key :type Key%20Structure :default "None"))
  (:Pressed
    (if (Variables|Default|GetInCar)
      (Collision|SetActorEnableCollision true)
      (Rendering|SetActorHiddenInGame false)
      (Transformation|DetachFromActor "KeepWorld" "KeepWorld" "KeepWorld")
      (Variables|Default|SetInCar false)
      (Variables|/Game/_Dowan/Vehicle/BP_Vehicle_SUV.BP_Vehicle_SUV_C|SetSeat2 (Variables|Default|GetAs%20BP%20Vehicle%20SUV) false)
      (elif (Variables|Default|GetVehicletest)
        (Variables|Default|SetInCar true)
        (CallFunction|VehicleServer)))))

(fn ConstructionScript)

(fn ReloadPistol
  (bind _equipweapon (Variables|Default|GetEquipWeapon))
  (bind _asbp_pistol (Utilities|Casting|CastToBP_Pistol _equipweapon))
  (if (> (Variables|/Script/YGL_MultiProject.WeaponBase|GetMaxAmmo _equipweapon) 0)
    (if (not (== 10 (Variables|/Script/YGL_MultiProject.WeaponBase|GetCurAmmo _equipweapon)))
      (if (>= (Variables|/Script/YGL_MultiProject.WeaponBase|GetMaxAmmo _equipweapon) 10)
        (Variables|/Script/YGL_MultiProject.WeaponBase|SetMaxAmmo _asbp_pistol (Math|Integer|Clamp(Integer) (- (Variables|/Script/YGL_MultiProject.WeaponBase|GetMaxAmmo _asbp_pistol) (- 10 (Variables|/Script/YGL_MultiProject.WeaponBase|GetCurAmmo _equipweapon))) 0 30))
        (Variables|/Script/YGL_MultiProject.WeaponBase|SetCurAmmo _asbp_pistol (Math|Integer|Clamp(Integer) (+ (Variables|/Script/YGL_MultiProject.WeaponBase|GetCurAmmo _asbp_pistol) 10) 0 10))
        (else
          (Variables|Default|SetRestAmmo (Variables|/Script/YGL_MultiProject.WeaponBase|GetMaxAmmo _equipweapon))
          (Variables|/Script/YGL_MultiProject.WeaponBase|SetMaxAmmo _equipweapon (Math|Integer|Clamp(Integer) (- (Variables|/Script/YGL_MultiProject.WeaponBase|GetMaxAmmo _equipweapon) (- 10 (Variables|/Script/YGL_MultiProject.WeaponBase|GetCurAmmo _equipweapon))) 0 30))
          (Variables|/Script/YGL_MultiProject.WeaponBase|SetCurAmmo _equipweapon (Math|Integer|Clamp(Integer) (+ (Variables|/Script/YGL_MultiProject.WeaponBase|GetCurAmmo _equipweapon) (Variables|Default|GetRestAmmo)) 0 10)))))))

(fn ReloadRifle
  (bind _equipweapon (Variables|Default|GetEquipWeapon))
  (bind _asbp_rifle (Utilities|Casting|CastToBP_Rifle _equipweapon))
  (if (> (Variables|/Script/YGL_MultiProject.WeaponBase|GetMaxAmmo _equipweapon) 0)
    (if (not (== 30 (Variables|/Script/YGL_MultiProject.WeaponBase|GetCurAmmo _equipweapon)))
      (if (>= (Variables|/Script/YGL_MultiProject.WeaponBase|GetMaxAmmo _equipweapon) 30)
        (Variables|/Script/YGL_MultiProject.WeaponBase|SetMaxAmmo _asbp_rifle (Math|Integer|Clamp(Integer) (- (Variables|/Script/YGL_MultiProject.WeaponBase|GetMaxAmmo _asbp_rifle) (- 30 (Variables|/Script/YGL_MultiProject.WeaponBase|GetCurAmmo _equipweapon))) 0 150))
        (Variables|/Script/YGL_MultiProject.WeaponBase|SetCurAmmo _asbp_rifle (Math|Integer|Clamp(Integer) (+ (Variables|/Script/YGL_MultiProject.WeaponBase|GetCurAmmo _asbp_rifle) 30) 0 30))
        (else
          (Variables|Default|SetRestAmmo (Variables|/Script/YGL_MultiProject.WeaponBase|GetMaxAmmo _equipweapon))
          (Variables|/Script/YGL_MultiProject.WeaponBase|SetMaxAmmo _equipweapon (Math|Integer|Clamp(Integer) (- (Variables|/Script/YGL_MultiProject.WeaponBase|GetMaxAmmo _equipweapon) (- 30 (Variables|/Script/YGL_MultiProject.WeaponBase|GetCurAmmo _equipweapon))) 0 150))
          (Variables|/Script/YGL_MultiProject.WeaponBase|SetCurAmmo _equipweapon (Math|Integer|Clamp(Integer) (+ (Variables|/Script/YGL_MultiProject.WeaponBase|GetCurAmmo _equipweapon) (Variables|Default|GetRestAmmo)) 0 30)))))))

(fn ReloadSniper
  (bind _equipweapon (Variables|Default|GetEquipWeapon))
  (bind _asbp_sniper (Utilities|Casting|CastToBP_Sniper _equipweapon))
  (if (> (Variables|/Script/YGL_MultiProject.WeaponBase|GetMaxAmmo _equipweapon) 0)
    (if (not (== 5 (Variables|/Script/YGL_MultiProject.WeaponBase|GetCurAmmo _equipweapon)))
      (if (>= (Variables|/Script/YGL_MultiProject.WeaponBase|GetMaxAmmo _equipweapon) 5)
        (Variables|/Script/YGL_MultiProject.WeaponBase|SetMaxAmmo _asbp_sniper (Math|Integer|Clamp(Integer) (- (Variables|/Script/YGL_MultiProject.WeaponBase|GetMaxAmmo _asbp_sniper) (- 5 (Variables|/Script/YGL_MultiProject.WeaponBase|GetCurAmmo _equipweapon))) 0 15))
        (Variables|/Script/YGL_MultiProject.WeaponBase|SetCurAmmo _asbp_sniper (Math|Integer|Clamp(Integer) (+ (Variables|/Script/YGL_MultiProject.WeaponBase|GetCurAmmo _asbp_sniper) 5) 0 5))
        (else
          (Variables|Default|SetRestAmmo (Variables|/Script/YGL_MultiProject.WeaponBase|GetMaxAmmo _equipweapon))
          (Variables|/Script/YGL_MultiProject.WeaponBase|SetMaxAmmo _equipweapon (Math|Integer|Clamp(Integer) (- (Variables|/Script/YGL_MultiProject.WeaponBase|GetMaxAmmo _equipweapon) (- 5 (Variables|/Script/YGL_MultiProject.WeaponBase|GetCurAmmo _equipweapon))) 0 15))
          (Variables|/Script/YGL_MultiProject.WeaponBase|SetCurAmmo _equipweapon (Math|Integer|Clamp(Integer) (+ (Variables|/Script/YGL_MultiProject.WeaponBase|GetCurAmmo _equipweapon) (Variables|Default|GetRestAmmo)) 0 5)))))))

(fn ReloadShotgun
  (bind _equipweapon (Variables|Default|GetEquipWeapon))
  (bind _asbp_launcher (Utilities|Casting|CastToBP_Launcher _equipweapon))
  (if (> (Variables|/Script/YGL_MultiProject.WeaponBase|GetMaxAmmo _equipweapon) 0)
    (if (not (== 5 (Variables|/Script/YGL_MultiProject.WeaponBase|GetCurAmmo _equipweapon)))
      (if (>= (Variables|/Script/YGL_MultiProject.WeaponBase|GetMaxAmmo _equipweapon) 5)
        (Variables|/Script/YGL_MultiProject.WeaponBase|SetMaxAmmo _asbp_launcher (Math|Integer|Clamp(Integer) (- (Variables|/Script/YGL_MultiProject.WeaponBase|GetMaxAmmo _asbp_launcher) (- 5 (Variables|/Script/YGL_MultiProject.WeaponBase|GetCurAmmo _equipweapon))) 0 15))
        (Variables|/Script/YGL_MultiProject.WeaponBase|SetCurAmmo _asbp_launcher (Math|Integer|Clamp(Integer) (+ (Variables|/Script/YGL_MultiProject.WeaponBase|GetCurAmmo _asbp_launcher) 5) 0 5))
        (else
          (Variables|Default|SetRestAmmo (Variables|/Script/YGL_MultiProject.WeaponBase|GetMaxAmmo _equipweapon))
          (Variables|/Script/YGL_MultiProject.WeaponBase|SetMaxAmmo _equipweapon (Math|Integer|Clamp(Integer) (- (Variables|/Script/YGL_MultiProject.WeaponBase|GetMaxAmmo _equipweapon) (- 5 (Variables|/Script/YGL_MultiProject.WeaponBase|GetCurAmmo _equipweapon))) 0 15))
          (Variables|/Script/YGL_MultiProject.WeaponBase|SetCurAmmo _equipweapon (Math|Integer|Clamp(Integer) (+ (Variables|/Script/YGL_MultiProject.WeaponBase|GetCurAmmo _equipweapon) (Variables|Default|GetRestAmmo)) 0 5)))))))

(fn ReloadAmmo
  (Utilities|FlowControl|Sequence
    (:then_0
      (CallFunction|ReloadPistol))
    (:then_1
      (기본/디폴트|ReloadRifle))
    (:then_2
      (기본/디폴트|ReloadSniper))
    (:then_3
      (기본/디폴트|ReloadShotgun))))

(fn OnRepPotion
  (bind _asbp_main_hud (Utilities|Casting|CastToBP_MainHUD (HUD|GetHUD (Game|GetPlayerController 0))))
  (Default|UpdatePotion _asbp_main_hud))